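; BP_Weapon01 is a weapon actor whose Gun component can be attached to a BP_Hunter's hand.
; A custom event casts the actor's owner to BP_Hunter, caches it, and attaches Gun to the Hand01 socket on HunterBody.
; The Gun it attaches comes from a GetActorOfClass lookup for BP_Weapon01, rather than directly from this instance.
; BeginPlay caches the weapon itself through Gun's owner.
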(event Custom|CustomEvent
  (bind _asbp_hunter (Utilities|Casting|CastToBP_Hunter (Components|GetOwner)))
  (bind _returnvalue (Actor|GetActorOfClass "BP_Weapon01_C"))
  (bind _output_get (Variables|Default|SetBP_Hunter _asbp_hunter))
  (Transformation|AttachComponentToComponent (Variables|BP_Weapon01_C|GetGun _returnvalue) (Variables|/Game/SBS/BP_Hunter.BP_Hunter_C|GetHunterBody _output_get) "Hand01" "KeepRelative" "KeepRelative" "KeepRelative" true))

(event Collision|EventActorBeginOverlap
  (params (OtherActor :type Actor%20Object%20Reference)))

(event EventTick
  (params (DeltaSeconds :type Float%20%28single-precision%29)))

(event EventBeginPlay
  (bind _asbp_weapon_01 (Utilities|Casting|CastToBP_Weapon01 (Components|GetOwner (Variables|Default|GetGun))))
  (Variables|Default|SetBP_Weapon _asbp_weapon_01))

(fn ConstructionScript)